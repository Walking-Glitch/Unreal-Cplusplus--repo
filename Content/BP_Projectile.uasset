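; Projectile actor that kills a MyPawn it strikes.
; It turns its gravity scale up to full shortly after spawning, through a brief delay on BeginPlay.
; Sphere hit and overlap events share one path that calls Death on a MyPawn, or otherwise spawns a particle burst at the sphere and destroys the projectile.
; The projectile is not destroyed when it hits a MyPawn.
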(event `self.ReceiveBeginPlay`
  (`KismetSystemLibrary.Delay` 0.2)
  (set `ProjectileMovementComponent.ProjectileGravityScale` 1.0 (`self.ProjectileMovement`)))

(event `self.Sphere.OnComponentHit`
  (params (HitComponent :type "PrimitiveComponent Object Reference") (OtherActor :type "Actor Object Reference") (OtherComp :type "PrimitiveComponent Object Reference") (NormalImpulse :type "Vector Structure") (Hit :type "HitResult Structure (by ref)"))
  (bind _asmy_pawn (cast `MyPawn` (stale `self.Sphere.OnComponentBeginOverlap` OtherActor) :!label _label)
    (:`then`
      (`MyPawn.Death` _asmy_pawn))
    (:`CastFailed`
      (`GameplayStatics.SpawnEmitterAtLocation` "/Engine/Tutorial/SubEditors/TutorialAssets/TutorialParticleSystem.TutorialParticleSystem" (`SceneComponent.K2_GetComponentLocation` (`self.Sphere`)))
      (`self.K2_DestroyActor`))))

(event `self.Sphere.OnComponentBeginOverlap`
  (params (OverlappedComponent :type "PrimitiveComponent Object Reference") (OtherActor :type "Actor Object Reference") (OtherComp :type "PrimitiveComponent Object Reference") (OtherBodyIndex :type Integer) (bFromSweep :type Boolean) (SweepResult :type "HitResult Structure (by ref)"))
  (goto _label))

(fn `UserConstructionScript`)